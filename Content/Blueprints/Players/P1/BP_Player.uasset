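; Paper2D flipbook player character for a two-player game where wolves catch sheep and carry them to score.
; Enhanced Input drives movement, a cooldown-gated mask toggle that switches wolf form, and grabbing, which slows the carrier.
; Interface events flag catchable prey, award points, and teleport wolves back, respawning any carried sheep.
; Player 1 creates the HUD shared through BP_GMode and runs the countdown, which stores the winner and opens the ending level.
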(event Custom|Anim_HandleRotation
  ;[0.15 0.15 0.15 0.5] Rotation
  (Math|Float|CompareFloat (.y (Variables|/Script/Engine.MovementComponent|GetVelocity (Variables|Character|GetCharacterMovement))) 0.0
    (:>
      (Pawn|SetControlRotation (Pawn|GetController) (Math|Rotator|MakeRotator 0.0 0.0 1.8e+02)))
    (:==
      (if (Variables|Default|GetIs%20Moving%20Right)
        (Sprite|SetFlipbook (Variables|Default|GetPaperFlipbook) "/Game/Art/FPB_WolfIdle.FPB_WolfIdle")))
    (:<
      (Pawn|SetControlRotation (Pawn|GetController) (Math|Rotator|MakeRotator 0.0 0.0 0.0)))))

(event Custom|Anim_HandleAnim
  (bind _charactermovement (Variables|Character|GetCharacterMovement))
  (bind _velocity (Variables|/Script/Engine.MovementComponent|GetVelocity _charactermovement))
  (bind _returnvalue (> (.x _velocity) 0.0))
  ;[0.15 0.15 0.15 0.5] ANIM
  (if (Variables|STATES|GetIsWolf)
    (if (Variables|STATES|GetCarringSheep)
      (Sprite|SetFlipbook (Variables|Default|GetPaperFlipbook) (select _returnvalue "/Game/Art/FPB_WolfSheep_Down.FPB_WolfSheep_Down" "/Game/Art/FPB_WolfSheep_Up.FPB_WolfSheep_Up"))
      (else
        (Sprite|SetFlipbook (Variables|Default|GetPaperFlipbook) (select _returnvalue "/Game/Art/FPB_WolfDown.FPB_WolfDown" "/Game/Art/FPB_WolfUp.FPB_WolfUp"))))
    (else
      (Sprite|SetFlipbook (Variables|Default|GetPaperFlipbook) (select _returnvalue "/Game/Art/FPB_WolfDown1.FPB_WolfDown1" "/Game/Art/FPB_WolfUp1.FPB_WolfUp1")))))

(event Custom|RelojCall
  (params (Timer :type Float%20%28double-precision%29))
  ;[0.15 0.15 0.15 0.5] REloj
  (bind _returnvalue (Utilities|Time|SetTimerbyEvent (delegate Custom|AddSegs) 1.0 true)))

(event Custom|SoundSheepOnMouth
  (params (Condition :type Boolean))
  ;[0.15 0.15 0.15 0.5] SoundSheep
  (if (Variables|STATES|GetCarringSheep) :!label _label
    (bind _returnvalue (Audio|SpawnSound2D "/Game/Music/_sheep_bah._sheep_bah" 1.0 1.0 0.0 0))
    (Utilities|IsValid _returnvalue
      (:Is%20Valid
        (Utilities|FlowControl|Delay 2.0)
        (goto _label)))))

(event Custom|AddSegs
  ;[0.15 0.15 0.15 0.5] REloj
  (bind _output_get (Variables|Default|SetTimerSettings (- (Variables|Default|GetTimerSettings) 1.0)))
  (if (<= _output_get 0.0)
    (CallFunction|FnFinalGame)
    (Utilities|Time|ClearandInvalidateTimerbyHandle (stale Custom|RelojCall _returnvalue))
    (Utilities|FlowControl|Delay 0.5)
    (Game|OpenLevel(byName) "Lvl_Ending")
    (else
      (Default|FNStartClock (Variables|/Game/Blueprints/UI/UI_Main.UI_Main_C|GetUI_Clocl (Variables|Default|GetUI_Main)) _output_get))))

(event Input|EnhancedActionEvents|EnhancedInputActionIA_walkAD
  (params (ActionValue :type Float%20%28double-precision%29) (ElapsedSeconds :type Float%20%28double-precision%29) (TriggeredSeconds :type Float%20%28double-precision%29) (InputAction :type Input%20Action%20Object%20Reference :default "/Game/Blueprints/Players/P1/IA_walkAD.IA_walkAD"))
  ;[0.15 0.15 0.15 0.5] Movement
  (Pawn|Input|AddMovementInput (Math|Vector|MakeVector 0.0 ActionValue 0.0) 1.0 false)
  (CallFunction|AnimHandleAnim)
  (CallFunction|AnimHandleRotation))

(event Input|EnhancedActionEvents|EnhancedInputActionIA_WalkWS
  (params (ActionValue :type Float%20%28double-precision%29) (ElapsedSeconds :type Float%20%28double-precision%29) (TriggeredSeconds :type Float%20%28double-precision%29) (InputAction :type Input%20Action%20Object%20Reference :default "/Game/Blueprints/Players/P1/IA_WalkWS.IA_WalkWS"))
  ;[0.15 0.15 0.15 0.5] Movement
  (Pawn|Input|AddMovementInput (Math|Vector|MakeVector ActionValue 0.0 0.0) 1.0 false)
  (CallFunction|AnimHandleAnim)
  (CallFunction|AnimHandleRotation))

(event Input|EnhancedActionEvents|EnhancedInputActionIA_Mask
  (params (ActionValue :type Boolean) (ElapsedSeconds :type Float%20%28double-precision%29) (TriggeredSeconds :type Float%20%28double-precision%29) (InputAction :type Input%20Action%20Object%20Reference :default "/Game/Blueprints/Players/P1/IA_Mask.IA_Mask"))
  ;[0.15 0.15 0.15 0.5] Change Fase
  (:Started
    (if (not (Variables|STATES|GetCarringSheep))
      (if (Variables|Default|GetisOnCD)
        (Development|PrintString "IS ON CD")
        (else
          (Utilities|FlowControl|FlipFlop
            (:A
              (Variables|STATES|SetIsWolf false)
              (Input|DisableInput (Variables|Default|GetAs%20Player%20Controller))
              (Utilities|FlowControl|Delay 0.2)
              (Sprite|SetFlipbook (Variables|Default|GetPaperFlipbook) "/Game/Art/FPB_WolfMasking.FPB_WolfMasking")
              (Utilities|FlowControl|Delay 0.6)
              (Input|EnableInput (Variables|Default|GetAs%20Player%20Controller))
              (CallFunction|AnimHandleAnim))
            (:B
              (Variables|STATES|SetIsWolf true)
              (Input|DisableInput (Variables|Default|GetAs%20Player%20Controller))
              (Utilities|FlowControl|Delay 0.2)
              (Sprite|SetFlipbook (Variables|Default|GetPaperFlipbook) "/Game/Art/FPB_WolfMaskingRev.FPB_WolfMaskingRev")
              (Utilities|FlowControl|Delay 0.6)
              (Input|EnableInput (Variables|Default|GetAs%20Player%20Controller))
              (CallFunction|AnimHandleAnim)))
          (bind _p2 (CallFunction|IsP2?))
          (if _p2
            (Variables|Default|SetisOnCD true)
            (Utilities|FlowControl|Delay (Variables|Default|GetCDTransform))
            (Variables|Default|SetisOnCD false)
            (else
              (Variables|Default|SetisOnCD true)
              (Utilities|FlowControl|Delay (Variables|Default|GetCDTransform))
              (Variables|Default|SetisOnCD false))))))))

(event Input|EnhancedActionEvents|EnhancedInputActionIA_GetButton
  (params (ActionValue :type Boolean) (ElapsedSeconds :type Float%20%28double-precision%29) (TriggeredSeconds :type Float%20%28double-precision%29) (InputAction :type Input%20Action%20Object%20Reference :default "/Game/Blueprints/Players/P1/IA_GetButton.IA_GetButton"))
  (if (not (Variables|STATES|GetCarringSheep))
    (if (Variables|STATES|GetReadyToCatch)
      (Rendering|SetActorHiddenInGame (Variables|Default|GetPrey) true)
      (Collision|SetActorEnableCollision (Variables|Default|GetPrey) false)
      (Sprite|SetFlipbook (Variables|Default|GetPaperFlipbook) "/Paper2D/Tutorial/Paper2D/TutorialAssets/TutorialFlipBook.TutorialFlipBook")
      (Variables|STATES|SetCarringSheep true)
      (CallFunction|SoundSheeponMouth (Variables|STATES|GetCarringSheep))
      (Variables|/Script/Engine.CharacterMovementComponent|SetMaxWalkSpeed (Variables|Character|GetCharacterMovement) 4.5e+02))))

(event Input|EnhancedActionEvents|EnhancedInputActionIA_walkJoyLR
  (params (ActionValue :type Float%20%28double-precision%29) (ElapsedSeconds :type Float%20%28double-precision%29) (TriggeredSeconds :type Float%20%28double-precision%29) (InputAction :type Input%20Action%20Object%20Reference :default "/Game/Blueprints/Players/P1/IA_walkJoyLR.IA_walkJoyLR"))
  ;[0.15 0.15 0.15 0.5] Movement
  (Pawn|Input|AddMovementInput (Math|Vector|MakeVector 0.0 ActionValue 0.0) 1.0 false)
  (if (> (.y (Variables|/Script/Engine.MovementComponent|GetVelocity (Variables|Character|GetCharacterMovement))) 0.0)
    (Variables|Default|SetIs%20Moving%20Right true)
    (else
      (Variables|Default|SetIs%20Moving%20Right false)))
  (CallFunction|AnimHandleAnim)
  (CallFunction|AnimHandleRotation))

(event Input|EnhancedActionEvents|EnhancedInputActionIA_WalkJoyUPdown
  (params (ActionValue :type Float%20%28double-precision%29) (ElapsedSeconds :type Float%20%28double-precision%29) (TriggeredSeconds :type Float%20%28double-precision%29) (InputAction :type Input%20Action%20Object%20Reference :default "/Game/Blueprints/Players/P1/IA_WalkJoyUPdown.IA_WalkJoyUPdown"))
  ;[0.15 0.15 0.15 0.5] Movement
  (Pawn|Input|AddMovementInput (Math|Vector|MakeVector ActionValue 0.0 0.0) 1.0 false)
  (CallFunction|AnimHandleAnim)
  (CallFunction|AnimHandleRotation))

(event EventBeginPlay
  ;[0.15 0.15 0.15 0.5] Inputs SetUp
  (Utilities|FlowControl|Delay 0.1)
  (bind _asplayer_controller (Utilities|Casting|CastToPlayerController (Pawn|GetController)))
  (Variables|Default|SetAs%20Player%20Controller _asplayer_controller)
  (Utilities|IsValid (PlayerController|LocalPlayerSubsystems|GetEnhancedInputLocalPlayerSubsystem _asplayer_controller)
    (:Is%20Valid
      (Input|AddMappingContext (PlayerController|LocalPlayerSubsystems|GetEnhancedInputLocalPlayerSubsystem _asplayer_controller) "/Game/Blueprints/Players/P1/IA_mapping.IA_mapping" 0 "(bIgnoreAllPressedKeysUntilRelease=True,bForceImmediately=False,bNotifyUserSettings=False)")
      (bind _returnvalue (Actor|GetActorOfClass "/Game/Blueprints/Players/P1/BP_camP1.BP_camP1_C"))
      (Game|Player|SetViewTargetwithBlend (Variables|Default|GetAs%20Player%20Controller) _returnvalue 0.0 "VTBlend_Linear" 0.0 false)
      (Variables|Default|SetScore (Variables|Default|GetScoreInitial))
      (bind _p2 (CallFunction|IsP2?))
      (if _p2
        (bind _asbp_gmode (Utilities|Casting|CastToBP_GMode (Game|GetGameMode)))
        (bind _output_get (Variables|Default|SetUI_Main (Variables|/Game/Blueprints/BP_GMode.BP_GMode_C|GetUI_GM _asbp_gmode)))
        (Utilities|IsValid _output_get
          (:Is%20Valid
            (Default|SetPLayer2 _output_get self)))
        (else
          (bind _returnvalue_2 (UserInterface|CreateWidget "/Game/Blueprints/UI/UI_Main.UI_Main_C" 0 self))
          (bind _output_get_2 (Variables|Default|SetUI_Main _returnvalue_2))
          (UserInterface|Viewport|AddtoViewport _output_get_2 0)
          (bind _asbp_gmode_2 (Utilities|Casting|CastToBP_GMode (Game|GetGameMode)))
          (Variables|/Game/Blueprints/BP_GMode.BP_GMode_C|SetUI_GM _asbp_gmode_2 _output_get_2)
          (CallFunction|RelojCall 0.0))))))

(event EventBPITeleport
  (if (Variables|STATES|GetIsWolf)
    (Utilities|FlowControl|Sequence
      (:then_0
        (if (Variables|STATES|GetCarringSheep)
          (Game|SpawnActorfromClass "/Game/AI/Sheep/BP_Sheep.BP_Sheep_C" (Math|Transform|MakeTransform (Transformation|GetActorLocation) "0, 0, 0" "1.000000,1.000000,1.000000") "AlwaysSpawn" "MultiplyWithRoot" 0 0)
          (Variables|STATES|SetCarringSheep false)
          (Variables|/Script/Engine.CharacterMovementComponent|SetMaxWalkSpeed (Variables|Character|GetCharacterMovement) 8e+02)))
      (:then_1
        (Transformation|SetActorLocation "1070.000000,-50.000000,50.000000" false true)))))

(event EventBPIGetSheeps
  (params (Ovelap%20Sheep :type Boolean) (Sheeps :type Actor%20Object%20Reference))
  (if (and (Variables|STATES|GetIsWolf) Ovelap%20Sheep)
    (Variables|STATES|SetReadyToCatch true)
    (Variables|Default|SetPrey Sheeps)
    (else
      (Variables|STATES|SetReadyToCatch false)
      (Variables|Default|SetPrey 0))))

(event EventBPIScorepoint
  (bind _ui_main (Variables|Default|GetUI_Main))
  ;[0.15 0.15 0.15 0.5] Score
  (if (Variables|STATES|GetCarringSheep)
    (bind _output_get (Variables|Default|SetScore (+ (Variables|Default|GetScore) 1.0)))
    (CallFunction|FnResetForm)
    (bind _asbp_playercontroler (Utilities|Casting|CastToBP_Playercontroler (Pawn|GetController)))
    (if (Variables|/Game/Blueprints/Players/P1/BP_Playercontroler.BP_Playercontroler_C|GetP2 _asbp_playercontroler)
      (Default|RefreshScore (Variables|/Game/Blueprints/UI/UI_Main.UI_Main_C|GetUI_ScorePoints_2 _ui_main) _output_get)
      (Variables|Default|SetPuntosP2 _output_get)
      (else
        (Default|RefreshScore (Variables|/Game/Blueprints/UI/UI_Main.UI_Main_C|GetUI_ScorePoints _ui_main) _output_get)
        (Variables|Default|SetPuntosP1 _output_get)))))

(event Input|KeyboardEvents|Escape
  (params (Key :type Key%20Structure :default "None"))
  (:Pressed
    (Game|QuitGame 0 "Quit" false)))

(fn ConstructionScript)

(fn FnResetForm
  (Variables|STATES|SetIsWolf true)
  (Sprite|SetFlipbook (Variables|Default|GetPaperFlipbook) "/Game/Art/FPB_WolfDown.FPB_WolfDown")
  (Variables|STATES|SetReadyToCatch false)
  (Variables|STATES|SetCarringSheep false)
  (Variables|/Script/Engine.CharacterMovementComponent|SetMaxWalkSpeed (Variables|Character|GetCharacterMovement) 8e+02))

(fn IsP2?
  (bind _asbp_playercontroler (Utilities|Casting|CastToBP_Playercontroler (Pawn|GetController)))
  (if (Variables|/Game/Blueprints/Players/P1/BP_Playercontroler.BP_Playercontroler_C|GetP2 _asbp_playercontroler)
    (return true)
    (else
      (return false))))

(fn FnFinalGame
  (bind _returnvalue (Game|GetGameMode))
  (Widget|RemovefromParent (Variables|Default|GetUI_Main))
  (if (> (Variables|Default|GetPuntosP1) (Variables|Default|GetPuntosP2))
    (bind _asbp_gmode (Utilities|Casting|CastToBP_GMode _returnvalue))
    (Variables|/Game/Blueprints/BP_GMode.BP_GMode_C|SetWinner _asbp_gmode 1.0)
    (elif (> (Variables|Default|GetPuntosP2) (Variables|Default|GetPuntosP1))
      (bind _asbp_gmode_2 (Utilities|Casting|CastToBP_GMode _returnvalue))
      (Variables|/Game/Blueprints/BP_GMode.BP_GMode_C|SetWinner _asbp_gmode_2 2.0)
      (else
        (bind _asbp_gmode_3 (Utilities|Casting|CastToBP_GMode _returnvalue))
        (Variables|/Game/Blueprints/BP_GMode.BP_GMode_C|SetWinner _asbp_gmode_3 3.0)))))