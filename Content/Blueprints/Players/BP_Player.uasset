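; Player character that switches between wolf and sheep forms, catches sheep as the wolf and scores by delivering them.
; Enhanced Input drives planar movement, a mask toggle that swaps the Paper2D sprite, and a grab action; BeginPlay sets the view to a placed BP_camP1.
; Interface events flag catchable prey and award points.
; Grabbing hides the prey and slows movement until scoring resets the wolf form.
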(event Input|EnhancedActionEvents|EnhancedInputActionIA_walkAD
  (params (ActionValue :type Float%20%28double-precision%29) (ElapsedSeconds :type Float%20%28double-precision%29) (TriggeredSeconds :type Float%20%28double-precision%29) (InputAction :type Input%20Action%20Object%20Reference :default "/Game/Blueprints/Players/IA_walkAD.IA_walkAD"))
  ;[0.15 0.15 0.15 0.5] Movement
  (Pawn|Input|AddMovementInput (Math|Vector|MakeVector 0.0 ActionValue 0.0) 1.0 false))

(event Input|EnhancedActionEvents|EnhancedInputActionIA_WalkWS
  (params (ActionValue :type Float%20%28double-precision%29) (ElapsedSeconds :type Float%20%28double-precision%29) (TriggeredSeconds :type Float%20%28double-precision%29) (InputAction :type Input%20Action%20Object%20Reference :default "/Game/Blueprints/Players/IA_WalkWS.IA_WalkWS"))
  ;[0.15 0.15 0.15 0.5] Movement
  (Pawn|Input|AddMovementInput (Math|Vector|MakeVector ActionValue 0.0 0.0) 1.0 false))

(event Input|EnhancedActionEvents|EnhancedInputActionIA_Mask
  (params (ActionValue :type Boolean) (ElapsedSeconds :type Float%20%28double-precision%29) (TriggeredSeconds :type Float%20%28double-precision%29) (InputAction :type Input%20Action%20Object%20Reference :default "/Game/Blueprints/Players/IA_Mask.IA_Mask"))
  (bind _papersprite (Variables|Default|GetPaperSprite))
  ;[0.15 0.15 0.15 0.5] Change Fase
  (:Started
    (Utilities|FlowControl|FlipFlop
      (:A
        (Variables|Default|SetIsWolf true)
        (Rendering|Components|Sprite|SetSprite _papersprite "/Game/T_Wolf_Placeholder_Sprite.T_Wolf_Placeholder_Sprite"))
      (:B
        (Variables|Default|SetIsWolf false)
        (Rendering|Components|Sprite|SetSprite _papersprite "/Game/T_Sheep_Placeholder_Sprite.T_Sheep_Placeholder_Sprite")))))

(event Input|EnhancedActionEvents|EnhancedInputActionIA_GetButton
  (params (ActionValue :type Boolean) (ElapsedSeconds :type Float%20%28double-precision%29) (TriggeredSeconds :type Float%20%28double-precision%29) (InputAction :type Input%20Action%20Object%20Reference :default "/Game/Blueprints/Players/IA_GetButton.IA_GetButton"))
  (if (Variables|Default|GetReadyToCatch)
    (Rendering|SetActorHiddenInGame (Variables|Default|GetPrey) true)
    (Rendering|Components|Sprite|SetSprite (Variables|Default|GetPaperSprite) "/Game/SPRITE_SheepCatched.SPRITE_SheepCatched")
    (Variables|Default|SetCarringSheep true)
    (Variables|/Script/Engine.CharacterMovementComponent|SetMaxWalkSpeed (Variables|Character|GetCharacterMovement) 4.5e+02)))

(event EventBeginPlay
  (bind _asplayer_controller (Utilities|Casting|CastToPlayerController (Game|GetPlayerController 0)))
  (Utilities|IsValid (PlayerController|LocalPlayerSubsystems|GetEnhancedInputLocalPlayerSubsystem _asplayer_controller)
    (:Is%20Valid
      (Input|AddMappingContext (PlayerController|LocalPlayerSubsystems|GetEnhancedInputLocalPlayerSubsystem _asplayer_controller) "/Game/Blueprints/Players/IA_mapping.IA_mapping" 0 "(bIgnoreAllPressedKeysUntilRelease=True,bForceImmediately=False,bNotifyUserSettings=False)")
      (bind _returnvalue (Actor|GetActorOfClass "/Game/Blueprints/Players/BP_camP1.BP_camP1_C"))
      (Game|Player|SetViewTargetwithBlend (Game|GetPlayerController 0) _returnvalue 0.0 "VTBlend_Linear" 0.0 false)
      (Variables|Default|SetScore (Variables|Default|GetScoreInitial)))))

(event Collision|EventActorBeginOverlap
  (params (OtherActor :type Actor%20Object%20Reference)))

(event EventTick
  (params (DeltaSeconds :type Float%20%28single-precision%29)))

(event EventBPIGetSheeps
  (params (Ovelap%20Sheep :type Boolean) (Sheeps :type Actor%20Object%20Reference))
  (if (and (Variables|Default|GetIsWolf) Ovelap%20Sheep)
    (Variables|Default|SetReadyToCatch true)
    (Variables|Default|SetPrey Sheeps)
    (else
      (Variables|Default|SetReadyToCatch false)
      (Variables|Default|SetPrey 0))))

(event EventBPIScorepoint
  ;[0.15 0.15 0.15 0.5] Score
  (if (Variables|Default|GetCarringSheep)
    (bind _output_get (Variables|Default|SetScore (+ (Variables|Default|GetScore) 1.0)))
    (Development|PrintString (Utilities|String|ToString(Float) _output_get) true true "(R=1.000000,G=0.800990,B=0.149938,A=1.000000)" 5.0)
    (CallFunction|FnResetForm)))

(fn ConstructionScript)

(fn FnResetForm
  (Variables|Default|SetIsWolf true)
  (Rendering|Components|Sprite|SetSprite (Variables|Default|GetPaperSprite) "/Game/T_Wolf_Placeholder_Sprite.T_Wolf_Placeholder_Sprite")
  (Variables|Default|SetReadyToCatch false)
  (Variables|Default|SetCarringSheep false)
  (Variables|/Script/Engine.CharacterMovementComponent|SetMaxWalkSpeed (Variables|Character|GetCharacterMovement) 8e+02))