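; BP_Dog is a Paper2D dog character whose death trigger sends a teleport interface message to any actor that overlaps it.
; Tick snaps the flipbook sprite to one of two opposite world yaws, based on the actor's yaw.
; A separate animation event picks the down or up flipbook from X velocity, but nothing in this graph calls it.
; Control-rotation logic driven by Y velocity is left unconnected.
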(event OnComponentBeginOverlap(DeathTrigger)
  (params (OverlappedComponent :type Primitive%20Component%20Object%20Reference) (OtherActor :type Actor%20Object%20Reference) (OtherComp :type Primitive%20Component%20Object%20Reference) (OtherBodyIndex :type Integer) (bFromSweep :type Boolean) (SweepResult :type Hit%20Result%20Structure%20%28by%20ref%29))
  (Class|BPIPlayer|BPITeleport(Message) OtherActor))

(event Custom|Anim_HandleRotation
  (bind _paperflipbook (Variables|Default|GetPaperFlipbook))
  (if (> (.yaw (Transformation|GetActorRotation)) 15.0)
    (Transformation|SetWorldRotation _paperflipbook (Math|Rotator|MakeRotator 0.0 0.0 -9e+01) false false)
    (else
      (Transformation|SetWorldRotation _paperflipbook (Math|Rotator|MakeRotator 0.0 0.0 9e+01) false false))))

(event Custom|Anim_HandleAnim
  (Sprite|SetFlipbook (Variables|Default|GetPaperFlipbook) (select (> (.x (Variables|/Script/Engine.MovementComponent|GetVelocity (Variables|Character|GetCharacterMovement))) 0.0) "/Game/Art/FPB_DogDown.FPB_DogDown" "/Game/Art/FPB_DogUp.FPB_DogUp")))

(event EventBeginPlay)

(event Collision|EventActorBeginOverlap
  (params (OtherActor :type Actor%20Object%20Reference)))

(event EventTick
  (params (DeltaSeconds :type Float%20%28single-precision%29))
  (CallFunction|AnimHandleRotation))

(fn ConstructionScript)